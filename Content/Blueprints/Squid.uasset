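; Player-controlled squid character that swims on the X/Y plane and squirts ink behind itself, with its sprite component set to replicate.
; Boost, allowed only within a speed window, drops ink and adds a mass-scaled impulse along the current velocity, while Ink just spawns the ink actor.
; Tick turns the squid to face its velocity, caching the yaw at low speed to hold that facing once stopped.
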(event `self.ReceiveBeginPlay`
  (`ActorComponent.SetIsReplicated` (`self.Sprite`) true))

(event `self.ReceiveActorBeginOverlap`
  (params (OtherActor :type "Actor Object Reference")))

(event `InputAxis|MoveRight`
  (params (AxisValue :type "Float (single-precision)"))
  (`self.AddMovementInput` (1.0 0.0 0.0) AxisValue))

(event `InputAxis|MoveUp`
  (params (AxisValue :type "Float (single-precision)"))
  (`self.AddMovementInput` (0.0 1.0 0.0) AxisValue))

(event `InputAction|Boost`
  (bind _returnvalue (`self.GetVelocity`))
  (bind _returnvalue_2 (`KismetMathLibrary.VSize` _returnvalue))
  (:`Pressed`
    (if (and (>= _returnvalue_2 1.0) (<= _returnvalue_2 650.0))
      (`self.SpawnInk` "/Game/Blueprints/InkSprite.InkSprite_C")
      (`CharacterMovementComponent.AddImpulse` (`self.CharacterMovement`) (* _returnvalue (/ (`PrimitiveComponent.GetMass` (`self.CapsuleComponent`)) 5.0)) false))))

(event `InputAction|Ink`
  (:`Pressed`
    (`self.SpawnInk` "/Game/Blueprints/InkSprite.InkSprite_C")))

(event `self.ReceiveTick`
  (params (DeltaSeconds :type "Float (single-precision)"))
  (bind _returnvalue (`self.GetVelocity`))
  (bind _returnvalue_2 (`KismetMathLibrary.VSize` _returnvalue))
  (bind _returnvalue_3 (`KismetMathLibrary.MakeRot` 0.0 (`KismetMathLibrary.DegAtan2` (.y _returnvalue) (.x _returnvalue))))
  (if (and (<= _returnvalue_2 20.0) (> _returnvalue_2 8.0))
    (bind _output_get (set `self.Rotation` _returnvalue_3)))
  (`self.SetActorRotation` _returnvalue_3)
  (if (`KismetMathLibrary.NearlyEqual_FloatFloat` _returnvalue_2)
    (`self.SetActorRotation` _output_get)))

(fn `SpawnInk`
  (params (Ink :type "Actor Class Reference"))
  (bind _returnvalue (`|SpawnActorFromClass` Ink (`KismetMathLibrary.Conv_VectorToTransform` (`KismetMathLibrary.TransformLocation` (`self.GetTransform`) (-150.0 0.0 0.0)))))
  (`self.SetActorRotation` _returnvalue (`KismetMathLibrary.ComposeRotators` (`self.K2_GetActorRotation`) (struct :`Yaw` 90.0))))

(fn `UserConstructionScript`)